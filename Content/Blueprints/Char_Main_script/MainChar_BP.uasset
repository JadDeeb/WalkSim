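; MainChar_BP is the main character Blueprint, handling forward and sideways player movement.
; MoveForward and MoveRight axis inputs call AddMovementInput along forward and right vectors built only from control rotation yaw, so pitch and roll do not affect direction.
; A DisableMovement flag gates both axes, noted as blocking movement where no animation exists.
; RotateX, BeginPlay, Tick, overlap and construction script are empty.
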(event `InputAxis|MoveForward`
  (params (AxisValue :type "Float (single-precision)"))
  ;[1 1 1] Disable char movement where no anim exists
  (if (not (`self.DisableMovement`))
    (`self.AddMovementInput` (`KismetMathLibrary.GetForwardVector` (`KismetMathLibrary.MakeRotator` 0.0 0.0 (.yaw (`self.GetControlRotation`)))) AxisValue)))

(event `InputAxis|MoveRight`
  (params (AxisValue :type "Float (single-precision)"))
  ;[1 1 1] Disable char movement where no anim exists
  (if (not (`self.DisableMovement`))
    (`self.AddMovementInput` (`KismetMathLibrary.GetRightVector` (`KismetMathLibrary.MakeRotator` 0.0 0.0 (.yaw (`self.GetControlRotation`)))) AxisValue)))

(event `InputAxis|RotateX`
  (params (AxisValue :type "Float (single-precision)")))

(fn `UserConstructionScript`)